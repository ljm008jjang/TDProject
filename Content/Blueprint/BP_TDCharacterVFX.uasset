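; BP_TDCharacterVFX is a character Blueprint that drives the cutout location of the fog-of-war effect.
; Every Tick, it looks up BP_FogOfWarVFX with GetActorOfClass and sends it the Mesh world location through UpdateCutoutLocationMessage.
; An unconnected alternative, PlaneActorMethod, line traces from Camera to Mesh and sends the hit location to the hit actor, with a separate unused debug sphere.
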(event `self.ReceiveTick`
  (params (DeltaSeconds :type "Float (single-precision)"))
  (bind _returnvalue (`GameplayStatics.GetActorOfClass` "/Game/Blueprint/BP_FogOfWarVFX.BP_FogOfWarVFX_C"))
  (message `FogOfWarInterface.UpdateCutoutLocation` _returnvalue (`SceneComponent.K2_GetComponentLocation` (`self.Mesh`))))

(fn `UserConstructionScript`)