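; Actor component that controls its owner's fog-of-war visibility, hiding the owner in game on BeginPlay.
; At start it caches dynamic material instances from the owner's skeletal mesh, creating and assigning them where needed.
; EventSetFOWHidden shows or hides the owner and writes the current game time to each material's StartTime parameter, giving shaders a timestamp for each visibility update.
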(event `self.ReceiveBeginPlay`
  (bind _returnvalue (`self.GetOwner`))
  (bind _returnvalue_2 (`Actor.GetComponentByClass` _returnvalue "/Script/Engine.SkeletalMeshComponent"))
  (bind _output_get (set `self.Owner` _returnvalue))
  (`Actor.SetActorHiddenInGame` _output_get true)
  (`/Engine/EditorBlueprintResources/StandardMacros.IsValid` _returnvalue_2
    (:`Is Valid`
      (for (_array_element _array_index) (`MeshComponent.GetMaterials` _returnvalue_2)
        (bind _asmaterial_instance_dynamic (cast `MaterialInstanceDynamic` _array_element)
          (:`then`
            (`KismetArrayLibrary.Array_Add` (`self.MIDs`) _asmaterial_instance_dynamic))
          (:`CastFailed`
            (bind _returnvalue_3 (`KismetMaterialLibrary.CreateDynamicMaterialInstance` _array_element))
            (`KismetArrayLibrary.Array_Add` (`self.MIDs`) _returnvalue_3)
            (`PrimitiveComponent.SetMaterial` _returnvalue_2 _array_index _returnvalue_3)))))))

(event `EventSetFOWHidden`
  (params (bIsHidden :type Boolean))
  (bind _owner (`self.Owner`))
  (`/Engine/EditorBlueprintResources/StandardMacros.IsValid` _owner
    (:`Is Valid`
      (`Actor.SetActorHiddenInGame` _owner bIsHidden)
      (for _array_element (`self.MIDs`)
        (`MaterialInstanceDynamic.SetScalarParameterValue` _array_element "StartTime" (`KismetSystemLibrary.GetGameTimeInSeconds`))))))